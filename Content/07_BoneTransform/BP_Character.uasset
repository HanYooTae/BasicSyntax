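; BP_Character is a character Blueprint that computes a head pitch angle toward a Target actor, apparently for a bone transform.
; Each Tick it takes the arccosine of the dot product between the actor's up vector and the normalized direction from the head socket to Target.
; That angle, offset to be relative to horizontal and clamped to a symmetric limit, is stored in Pitch.
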(event EventBeginPlay)

(event Collision|EventActorBeginOverlap
  (params (OtherActor :type Actor%20Object%20Reference)))

(event EventTick
  (params (DeltaSeconds :type Float%20%28single-precision%29))
  (Variables|Default|SetPitch (Math|Float|Clamp(Float) (+ (Class|KismetMathLibrary|DegAcos (Math|Vector|DotProduct (Transformation|GetActorUpVector) (Math|Vector|Normalize (- (Transformation|GetActorLocation (Variables|Default|GetTarget)) (Transformation|GetSocketLocation (Variables|Character|GetMesh) "head"))))) -9e+01) -3e+01 3e+01)))

(fn ConstructionScript)